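; BP_Item is a generic item Blueprint that configures itself from the DT_Items data table.
; Its construction script looks up the row named by ItemIdentificator and always copies the base info, plus weapon, armor or arrow info according to ItemType.
; The row's preview widget feeds ItemWidgetComponent, and debug prints show the item name or flag an unknown row.
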(fn `UserConstructionScript`
  (bind _returnvalue (`|GetDataTableRow` "/Game/MORPG/Blueprints/Data/DT_Items.DT_Items" (`self.ItemIdentificator`))
    (:`then`
      (bind (_itemtype _baseinfo _weaponinfo _armorinfo _arrowinfo) (break `/Game/MORPG/Blueprints/Data/S_ItemData` _returnvalue))
      (switch `EItemType` _itemtype
        (:`Item`
          _)
        (:`Weapon`
          (set `self.WeaponInfo` _weaponinfo))
        (:`Armor`
          (set `self.ArmorInfo` _armorinfo))
        (:`Arrow`
          (set `self.ArrowInfo` _arrowinfo)))
      (bind _output_get (set `self.ItemInfo` _baseinfo))
      (bind (_itemid _itemname _itemmesh _itemicon _pickupsound _pickupfx _dropfx _bisstackable _count _cost _weight _itempreviewwidget) (break `ItemInfo` _output_get))
      (`WidgetComponent.SetWidget` (`self.ItemWidgetComponent`) _itempreviewwidget)
      (`KismetSystemLibrary.PrintString` (`KismetTextLibrary.Conv_TextToString` (`KismetTextLibrary.Conv_NameToText` _itemname))))
    (:`RowNotFound`
      (`KismetSystemLibrary.PrintString` "UNKNOW ITEM" true true (struct :`R` 1.0 :`A` 1.0) 5.0))))